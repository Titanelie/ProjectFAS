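; Animated floating crystal prop that spins on its vertical axis while its top mesh and six crystal meshes swivel and bob.
; Construction Script derives two tilted swivel axes, which Tick rotates by advancing angles into one wobble rotation shared by all seven meshes.
; MakeSine advances each crystal's own phase and MakeBobbing turns it into a sine Z offset from a base location, with the top mesh using equivalent inline math.
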(event EventBeginPlay)

(event Collision|EventActorBeginOverlap
  (params (OtherActor :type Actor%20Object%20Reference)))

(event EventTick
  (params (DeltaSeconds :type Float%20%28single-precision%29))
  (bind _returnvalue (* DeltaSeconds 3.6e+02))
  (bind _topmesh (Variables|Default|GetTopMesh))
  (Transformation|AddActorLocalRotation (Math|Vector|RotatorfromAxisandAngle "0, 0,1.000000" (* DeltaSeconds (Variables|Default|GetRotationSpeed))) false false)
  ;[0 0 0] Progress swivel angle
  (Variables|SwivelTopMesh|SetCurrent%20Swivel%20X (Math|Float|%(Float) (+ (/ _returnvalue (Variables|SwivelTopMesh|GetSwivel%20Cone%20X)) (Variables|SwivelTopMesh|GetCurrent%20Swivel%20X)) 3.6e+02))
  (Variables|SwivelTopMesh|SetCurrent%20Swivel%20Y (Math|Float|%(Float) (+ (/ _returnvalue (Variables|SwivelTopMesh|GetSwivel%20Cone%20Y)) (Variables|SwivelTopMesh|GetCurrent%20Swivel%20Y)) 3.6e+02))
  (Utilities|FlowControl|Sequence
    (:then_0
      (Transformation|SetRelativeRotation _topmesh (Math|Rotator|MakeRotfromXY (Math|Vector|RotateVectorAroundAxis (Variables|SwivelTopMesh|GetSwivel%20Axis%20X) (Variables|SwivelTopMesh|GetCurrent%20Swivel%20X) "1.000000, 0, 0") (Math|Vector|RotateVectorAroundAxis (Variables|SwivelTopMesh|GetSwivel%20Axis%20Y) (Variables|SwivelTopMesh|GetCurrent%20Swivel%20Y) "0,1.000000, 0")) false false)
      (Utilities|FlowControl|Sequence
        (:then_0
          ;[0 0 0] Progress bobbing cycles
          (Variables|Bobbing|SetBobbing%20Cycle%201 (Math|Float|%(Float) (+ (Variables|Bobbing|GetBobbing%20Cycle%201) (/ (* (Utilities|Time|GetWorldDeltaSeconds) 3.6e+02) (Variables|Bobbing|GetBobbing%20Period%201))) 3.6e+02)))
        (:then_3
          (Transformation|SetRelativeLocation _topmesh (+ (Variables|Bobbing|GetTopMesh_Location) (Math|Vector|MakeVector 0.0 0.0 (* (Variables|Bobbing|GetBobbing%20Amplitude%201) (Math|Trig|Sin(Degrees) (Variables|Bobbing|GetBobbing%20Cycle%201))))) false false)
          ;[0 0 0] Crystall_A_MakeAnim
          (bind _newparam (CallFunction|MakeSine (Variables|Crystall_A|GetCrystall_A_period) (Variables|Crystall_A|GetCrystall_A_cycle)))
          (bind _output_get (Variables|Crystall_A|SetCrystall_A_cycle _newparam))
          (bind _z_bobbing (CallFunction|MakeBobbing (Variables|Crystall_A|GetCrystall_A_amplitude) _output_get))
          (Transformation|SetRelativeLocation (Variables|Default|GetT_Crystall_02_A) (+ (Variables|CrystallVectors|GetCrystall_A) (Math|Vector|MakeVector 0.0 0.0 _z_bobbing)) false false)
          ;[0 0 0] Crystall_C_MakeAnim
          (bind _newparam_2 (CallFunction|MakeSine (Variables|Crystall_C|GetCrystall_C%20Period) (Variables|Crystall_C|GetCrystall_C%20Cycle)))
          (bind _output_get_2 (Variables|Crystall_C|SetCrystall_C%20Cycle _newparam_2))
          (bind _z_bobbing_2 (CallFunction|MakeBobbing (Variables|Crystall_C|GetCrystall_C%20Amplitude) _output_get_2))
          (Transformation|SetRelativeLocation (Variables|Default|GetT_Crystall_02_C) (+ (Variables|CrystallVectors|GetCrystall_C) (Math|Vector|MakeVector 0.0 0.0 _z_bobbing_2)) false false)
          ;[0 0 0] Crystall_D_MakeAnim
          (bind _newparam_3 (CallFunction|MakeSine (Variables|Crystall_D|GetCrystall_D%20Period) (Variables|Crystall_D|GetCrystall_D%20Cycle)))
          (bind _output_get_3 (Variables|Crystall_D|SetCrystall_D%20Cycle _newparam_3))
          (bind _z_bobbing_3 (CallFunction|MakeBobbing (Variables|Crystall_D|GetCrystall_D%20Amplitude) _output_get_3))
          (Transformation|SetRelativeLocation (Variables|Default|GetT_Crystall_02_D) (+ (Variables|CrystallVectors|GetCrystall_D) (Math|Vector|MakeVector 0.0 0.0 _z_bobbing_3)) false false)
          ;[0 0 0] Crystall_E_MakeAnim
          (bind _newparam_4 (CallFunction|MakeSine (Variables|Crystall_E|GetCrystall_E%20Period) (Variables|Crystall_E|GetCrystall_E%20Cycle)))
          (bind _output_get_4 (Variables|Crystall_E|SetCrystall_E%20Cycle _newparam_4))
          (bind _z_bobbing_4 (CallFunction|MakeBobbing (Variables|Crystall_E|GetCrystall_E%20Amplitude) _output_get_4))
          (Transformation|SetRelativeLocation (Variables|Default|GetT_Crystall_02_E) (+ (Variables|CrystallVectors|GetCrystall_E) (Math|Vector|MakeVector 0.0 0.0 _z_bobbing_4)) false false)
          ;[0 0 0] Crystall_F_MakeAnim
          (bind _newparam_5 (CallFunction|MakeSine (Variables|Crystall_F|GetCrystall_F%20Period) (Variables|Crystall_F|GetCrystall_F%20Cycle)))
          (bind _output_get_5 (Variables|Crystall_F|SetCrystall_F%20Cycle _newparam_5))
          (bind _z_bobbing_5 (CallFunction|MakeBobbing (Variables|Crystall_F|GetCrystall_F%20Amplitude) _output_get_5))
          (Transformation|SetRelativeLocation (Variables|Default|GetT_Crystall_02_F) (+ (Variables|CrystallVectors|GetCrystall_F) (Math|Vector|MakeVector 0.0 0.0 _z_bobbing_5)) false false)
          ;[0 0 0] Crystall_G_MakeAnim
          (bind _newparam_6 (CallFunction|MakeSine (Variables|Crystall_G|GetCrystall_G%20Period) (Variables|Crystall_G|GetCrystall_G%20Cycle)))
          (bind _output_get_6 (Variables|Crystall_G|SetCrystall_G%20Cycle _newparam_6))
          (bind _z_bobbing_6 (CallFunction|MakeBobbing (Variables|Crystall_G|GetCrystall_G%20Amplitude) _output_get_6))
          (Transformation|SetRelativeLocation (Variables|Default|GetT_Crystall_02_G) (+ (Variables|CrystallVectors|GetCrystall_G) (Math|Vector|MakeVector 0.0 0.0 _z_bobbing_6)) false false))))
    (:then_1
      (Transformation|SetRelativeRotation (Variables|Default|GetT_Crystall_02_A) (Math|Rotator|MakeRotfromXY (Math|Vector|RotateVectorAroundAxis (Variables|SwivelTopMesh|GetSwivel%20Axis%20X) (Variables|SwivelTopMesh|GetCurrent%20Swivel%20X) "1.000000, 0, 0") (Math|Vector|RotateVectorAroundAxis (Variables|SwivelTopMesh|GetSwivel%20Axis%20Y) (Variables|SwivelTopMesh|GetCurrent%20Swivel%20Y) "0,1.000000, 0")) false false))
    (:then_2
      (Transformation|SetRelativeRotation (Variables|Default|GetT_Crystall_02_C) (Math|Rotator|MakeRotfromXY (Math|Vector|RotateVectorAroundAxis (Variables|SwivelTopMesh|GetSwivel%20Axis%20X) (Variables|SwivelTopMesh|GetCurrent%20Swivel%20X) "1.000000, 0, 0") (Math|Vector|RotateVectorAroundAxis (Variables|SwivelTopMesh|GetSwivel%20Axis%20Y) (Variables|SwivelTopMesh|GetCurrent%20Swivel%20Y) "0,1.000000, 0")) false false))
    (:then_3
      (Transformation|SetRelativeRotation (Variables|Default|GetT_Crystall_02_D) (Math|Rotator|MakeRotfromXY (Math|Vector|RotateVectorAroundAxis (Variables|SwivelTopMesh|GetSwivel%20Axis%20X) (Variables|SwivelTopMesh|GetCurrent%20Swivel%20X) "1.000000, 0, 0") (Math|Vector|RotateVectorAroundAxis (Variables|SwivelTopMesh|GetSwivel%20Axis%20Y) (Variables|SwivelTopMesh|GetCurrent%20Swivel%20Y) "0,1.000000, 0")) false false))
    (:then_4
      (Transformation|SetRelativeRotation (Variables|Default|GetT_Crystall_02_E) (Math|Rotator|MakeRotfromXY (Math|Vector|RotateVectorAroundAxis (Variables|SwivelTopMesh|GetSwivel%20Axis%20X) (Variables|SwivelTopMesh|GetCurrent%20Swivel%20X) "1.000000, 0, 0") (Math|Vector|RotateVectorAroundAxis (Variables|SwivelTopMesh|GetSwivel%20Axis%20Y) (Variables|SwivelTopMesh|GetCurrent%20Swivel%20Y) "0,1.000000, 0")) false false))
    (:then_5
      (Transformation|SetRelativeRotation (Variables|Default|GetT_Crystall_02_F) (Math|Rotator|MakeRotfromXY (Math|Vector|RotateVectorAroundAxis (Variables|SwivelTopMesh|GetSwivel%20Axis%20X) (Variables|SwivelTopMesh|GetCurrent%20Swivel%20X) "1.000000, 0, 0") (Math|Vector|RotateVectorAroundAxis (Variables|SwivelTopMesh|GetSwivel%20Axis%20Y) (Variables|SwivelTopMesh|GetCurrent%20Swivel%20Y) "0,1.000000, 0")) false false))
    (:then_6
      (Transformation|SetRelativeRotation (Variables|Default|GetT_Crystall_02_G) (Math|Rotator|MakeRotfromXY (Math|Vector|RotateVectorAroundAxis (Variables|SwivelTopMesh|GetSwivel%20Axis%20X) (Variables|SwivelTopMesh|GetCurrent%20Swivel%20X) "1.000000, 0, 0") (Math|Vector|RotateVectorAroundAxis (Variables|SwivelTopMesh|GetSwivel%20Axis%20Y) (Variables|SwivelTopMesh|GetCurrent%20Swivel%20Y) "0,1.000000, 0")) false false))))

(fn ConstructionScript
  (Variables|SwivelTopMesh|SetSwivel%20Axis%20X (Math|Vector|RotateVectorAroundAxis "1.000000, 0, 0" (Variables|SwivelTopMesh|GetSwivel%20Cone%20X) "0, 0,1.000000"))
  (Variables|SwivelTopMesh|SetSwivel%20Axis%20Y (Math|Vector|RotateVectorAroundAxis "0.000000,1.000000, 0" (Variables|SwivelTopMesh|GetSwivel%20Cone%20Y) "0, 0,1.000000")))

(fn MakeSine
  (params (Period :type Float%20%28single-precision%29) (Cycle :type Float%20%28single-precision%29))
  (return (Math|Float|%(Float) (+ Cycle (/ (* (Utilities|Time|GetWorldDeltaSeconds) 3.6e+02) Period)) 3.6e+02)))

(fn MakeBobbing
  (params (Amplitude :type Float%20%28single-precision%29) (Cycle :type Float%20%28single-precision%29))
  (return (* Amplitude (Math|Trig|Sin(Degrees) Cycle))))