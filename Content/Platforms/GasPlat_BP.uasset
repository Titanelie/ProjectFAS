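; Gas platform actor that pushes the player character along the platform's up vector while they are within its range.
; Overlap events with the third-person character set a flag, and Tick applies a movement force scaled by GasStrength to player 0 while it is set.
; The construction script sizes the Range box from configurable dimensions and raises it by its half-height so the volume extends upward from the actor's origin.
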(event EventTick
  (params (DeltaSeconds :type Float%20%28single-precision%29))
  (if (Variables|Default|GetIsOverlapping)
    (Physics|AddForce (Variables|/Script/Engine.Character|GetCharacterMovement (Game|GetPlayerCharacter 0)) (* (Transformation|GetActorUpVector) (Variables|Default|GetGasStrength)))))

(event Collision|EventActorEndOverlap
  (params (OtherActor :type Actor%20Object%20Reference))
  (Utilities|Casting|CastToBP_ThirdPersonCharacter OtherActor)
  (Variables|Default|SetIsOverlapping false))

(event Collision|EventActorBeginOverlap
  (params (OtherActor :type Actor%20Object%20Reference))
  (Utilities|Casting|CastToBP_ThirdPersonCharacter OtherActor)
  (Variables|Default|SetIsOverlapping true))

(fn ConstructionScript
  (Components|Box|SetBoxExtent (Variables|Default|GetRange) (Math|Vector|MakeVector (/ (Variables|Default|GetRangeX) 2.0) (/ (Variables|Default|GetRangeY) 2.0) (/ (Variables|Default|GetRangeZ) 2.0)) true)
  (Transformation|SetRelativeLocation (Variables|Default|GetRange) (Math|Vector|MakeVector 0.0 0.0 (.z (Variables|/Script/Engine.BoxComponent|GetBoxExtent (Variables|Default|GetRange)))) false false))