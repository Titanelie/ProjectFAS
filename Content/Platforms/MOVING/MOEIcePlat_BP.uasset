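; Moving ice platform that travels from its start location to a set end location after the player character enters its Falling trigger.
; Overlap begin waits two seconds, then plays a timeline that lerps the Ice component's relative location.
; Overlap end waits the same delay, then reverses it, with DurationInSeconds setting the play rate.
; The construction script places EndPlat at EndLocation, marking the destination.
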(event OnComponentBeginOverlap(Falling)
  (params (OverlappedComponent :type Primitive%20Component%20Object%20Reference) (OtherActor :type Actor%20Object%20Reference) (OtherComp :type Primitive%20Component%20Object%20Reference) (OtherBodyIndex :type Integer) (bFromSweep :type Boolean) (SweepResult :type Hit%20Result%20Structure%20%28by%20ref%29))
  (Utilities|Casting|CastToBP_ThirdPersonCharacter OtherActor)
  (Utilities|FlowControl|Delay 2.0)
  (Components|Timeline|SetPlayRate (Variables|Default|GetMovePlatform) (/ 1.0 (Variables|Default|GetDuration%20%28In%20Seconds%29)))
  (bind _moveplatform (Timeline|MovePlatform Play)
    (:Update
      (Transformation|SetRelativeLocation (Variables|Default|GetIce) (Math|Vector|Lerp(Vector) (Variables|Default|GetStart%20Location) (Variables|Default|GetEnd%20Location) _moveplatform) false false))))

(event OnComponentEndOverlap(Falling)
  (params (OverlappedComponent :type Primitive%20Component%20Object%20Reference) (OtherActor :type Actor%20Object%20Reference) (OtherComp :type Primitive%20Component%20Object%20Reference) (OtherBodyIndex :type Integer))
  (Utilities|Casting|CastToBP_ThirdPersonCharacter OtherActor)
  (Utilities|FlowControl|Delay 2.0)
  (Components|Timeline|SetPlayRate (Variables|Default|GetMovePlatform) (/ 1.0 (Variables|Default|GetDuration%20%28In%20Seconds%29)))
  (bind _moveplatform (Timeline|MovePlatform Reverse)
    (:Update
      (Transformation|SetRelativeLocation (Variables|Default|GetIce) (Math|Vector|Lerp(Vector) (Variables|Default|GetStart%20Location) (Variables|Default|GetEnd%20Location) _moveplatform) false false))))

(event EventBeginPlay
  (Variables|Default|SetStart%20Location (Variables|/Script/Engine.SceneComponent|GetRelativeLocation (Variables|Default|GetIce))))

(fn ConstructionScript
  (Transformation|SetRelativeLocation (Variables|Default|GetEndPlat) (Variables|Default|GetEnd%20Location) false false))