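; Moving gas platform that pushes the third-person character along the actor's up vector while it overlaps the actor.
; Overlap events toggle a flag, and Tick applies the force to the player's movement component while it is set.
; Entering or leaving the Range box plays or reverses, after a delay, a duration-scaled timeline lerping GasPlat between start and end locations.
; The construction script sizes and raises Range and positions EndPlatGAS at the end location.
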(event OnComponentBeginOverlap(Range)
  (params (OverlappedComponent :type Primitive%20Component%20Object%20Reference) (OtherActor :type Actor%20Object%20Reference) (OtherComp :type Primitive%20Component%20Object%20Reference) (OtherBodyIndex :type Integer) (bFromSweep :type Boolean) (SweepResult :type Hit%20Result%20Structure%20%28by%20ref%29))
  (Utilities|Casting|CastToBP_ThirdPersonCharacter OtherActor)
  (Utilities|FlowControl|Delay 1.0)
  (Components|Timeline|SetPlayRate (Variables|Default|GetMovePlatGAS) (/ 1.0 (Variables|Default|GetDuration%20%28gasSEC%29)))
  (bind _moveplatform (Timeline|MovePlatGAS Play)
    (:Update
      (Transformation|SetRelativeLocation (Variables|Default|GetGasPlat) (Math|Vector|Lerp(Vector) (Variables|Default|GetStart%20Location%20GAS) (Variables|Default|GetEnd%20Location%20GAS) _moveplatform) false false))))

(event OnComponentEndOverlap(Range)
  (params (OverlappedComponent :type Primitive%20Component%20Object%20Reference) (OtherActor :type Actor%20Object%20Reference) (OtherComp :type Primitive%20Component%20Object%20Reference) (OtherBodyIndex :type Integer))
  (Utilities|Casting|CastToBP_ThirdPersonCharacter OtherActor)
  (Utilities|FlowControl|Delay 1.0)
  (Components|Timeline|SetPlayRate (Variables|Default|GetMovePlatGAS) (/ 1.0 (Variables|Default|GetDuration%20%28gasSEC%29)))
  (bind _moveplatform (Timeline|MovePlatGAS Reverse)
    (:Update
      (Transformation|SetRelativeLocation (Variables|Default|GetGasPlat) (Math|Vector|Lerp(Vector) (Variables|Default|GetStart%20Location%20GAS) (Variables|Default|GetEnd%20Location%20GAS) _moveplatform) false false))))

(event EventBeginPlay
  (Variables|Default|SetStart%20Location%20GAS (Variables|/Script/Engine.SceneComponent|GetRelativeLocation (Variables|Default|GetGasPlat))))

(event EventTick
  (params (DeltaSeconds :type Float%20%28single-precision%29))
  (if (Variables|Default|GetIsOverlapping)
    (Physics|AddForce (Variables|/Script/Engine.Character|GetCharacterMovement (Game|GetPlayerCharacter 0)) (* (Transformation|GetActorUpVector) (Variables|Default|GetGasStrength)))))

(event Collision|EventActorEndOverlap
  (params (OtherActor :type Actor%20Object%20Reference))
  (Utilities|Casting|CastToBP_ThirdPersonCharacter OtherActor)
  (Variables|Default|SetIsOverlapping false))

(event Collision|EventActorBeginOverlap
  (params (OtherActor :type Actor%20Object%20Reference))
  (Utilities|Casting|CastToBP_ThirdPersonCharacter OtherActor)
  (Variables|Default|SetIsOverlapping true))

(fn ConstructionScript
  (Components|Box|SetBoxExtent (Variables|Default|GetRange) (Math|Vector|MakeVector (/ (Variables|Default|GetRangeX) 2.0) (/ (Variables|Default|GetRangeY) 2.0) (/ (Variables|Default|GetRangeZ) 2.0)) true)
  (Transformation|SetRelativeLocation (Variables|Default|GetRange) (Math|Vector|MakeVector 0.0 0.0 (.z (Variables|/Script/Engine.BoxComponent|GetBoxExtent (Variables|Default|GetRange)))) false false)
  (Transformation|SetRelativeLocation (Variables|Default|GetEndPlatGAS) (Variables|Default|GetEnd%20Location%20GAS) false false))