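; MOVPlatChange_BP is a platform actor with Gass and Ice change fields and a Water bounce volume.
; Each field opens a Gate while BP_ThirdPersonCharacter overlaps it, letting its Activate input through after a short delay.
; The Gass and Ice actions currently only print their names.
; Any overlap with Water launches player 0's character straight up, overriding vertical velocity.
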(event OnComponentBeginOverlap(Water)
  (params (OverlappedComponent :type Primitive%20Component%20Object%20Reference) (OtherActor :type Actor%20Object%20Reference) (OtherComp :type Primitive%20Component%20Object%20Reference) (OtherBodyIndex :type Integer) (bFromSweep :type Boolean) (SweepResult :type Hit%20Result%20Structure%20%28by%20ref%29))
  (Character|LaunchCharacter (Game|GetPlayerCharacter 0) "0, 0,1000.000000" false true))

(event OnComponentEndOverlap(PlatChangeFieldGass)
  (params (OverlappedComponent :type Primitive%20Component%20Object%20Reference) (OtherActor :type Actor%20Object%20Reference) (OtherComp :type Primitive%20Component%20Object%20Reference) (OtherBodyIndex :type Integer))
  (Utilities|Casting|CastToBP_ThirdPersonCharacter OtherActor)
  (Utilities|FlowControl|Gate true) ; enters at Close
)

(event OnComponentBeginOverlap(PlatChangeFieldGass)
  (params (OverlappedComponent :type Primitive%20Component%20Object%20Reference) (OtherActor :type Actor%20Object%20Reference) (OtherComp :type Primitive%20Component%20Object%20Reference) (OtherBodyIndex :type Integer) (bFromSweep :type Boolean) (SweepResult :type Hit%20Result%20Structure%20%28by%20ref%29))
  (Utilities|Casting|CastToBP_ThirdPersonCharacter OtherActor)
  (Utilities|FlowControl|Gate true) ; enters at Open
)

(event OnComponentBeginOverlap(PlatChangeFieldIce)
  (params (OverlappedComponent :type Primitive%20Component%20Object%20Reference) (OtherActor :type Actor%20Object%20Reference) (OtherComp :type Primitive%20Component%20Object%20Reference) (OtherBodyIndex :type Integer) (bFromSweep :type Boolean) (SweepResult :type Hit%20Result%20Structure%20%28by%20ref%29))
  (Utilities|Casting|CastToBP_ThirdPersonCharacter OtherActor)
  (Utilities|FlowControl|Gate true) ; enters at Open
)

(event OnComponentEndOverlap(PlatChangeFieldIce)
  (params (OverlappedComponent :type Primitive%20Component%20Object%20Reference) (OtherActor :type Actor%20Object%20Reference) (OtherComp :type Primitive%20Component%20Object%20Reference) (OtherBodyIndex :type Integer))
  (Utilities|Casting|CastToBP_ThirdPersonCharacter OtherActor)
  (Utilities|FlowControl|Gate true) ; enters at Close
)

(event EventBeginPlay
  (Input|EnableInput (Game|GetPlayerController 0)))

(event Input|ActionEvents|InputActionActivateIce
  (params (Key :type Key%20Structure))
  (:Pressed
    (Utilities|FlowControl|Delay 0.2)
    (Utilities|FlowControl|Gate true
      (:Exit
        (Development|PrintString "Ice")))))

(event Input|ActionEvents|InputActionActivateGass
  (params (Key :type Key%20Structure))
  (:Pressed
    (Utilities|FlowControl|Delay 0.2)
    (Utilities|FlowControl|Gate true
      (:Exit
        (Development|PrintString "Gass")))))

(fn ConstructionScript)